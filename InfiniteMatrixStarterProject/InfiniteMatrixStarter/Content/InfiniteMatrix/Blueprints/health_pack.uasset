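; Health pack pickup actor that heals the player on touch and removes itself.
; Both the actor overlap and the SM_Heart mesh overlap cast to BP_Player, call HealthUp and destroy the pack.
; Tick increments a Doomsday counter that destroys an uncollected pack after 1800 frames, so its lifetime depends on frame rate.
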(event OnComponentBeginOverlap(SM_Heart)
  (params (OverlappedComponent :type Primitive%20Component%20Object%20Reference) (OtherActor :type Actor%20Object%20Reference) (OtherComp :type Primitive%20Component%20Object%20Reference) (OtherBodyIndex :type Integer) (bFromSweep :type Boolean) (SweepResult :type Hit%20Result%20Structure%20%28by%20ref%29))
  (bind _asbp_player (Utilities|Casting|CastToBP_Player OtherActor))
  (Default|HealthUp _asbp_player)
  (Actor|DestroyActor))

(event EventBeginPlay)

(event Collision|EventActorBeginOverlap
  (params (OtherActor :type Actor%20Object%20Reference))
  (bind _asbp_player (Utilities|Casting|CastToBP_Player OtherActor))
  (Default|HealthUp _asbp_player)
  (Actor|DestroyActor))

(event EventTick
  (params (DeltaSeconds :type Float%20%28single-precision%29))
  (bind _output_get (Variables|Default|Setdoomsday (+ 1 (Variables|Default|Getdoomsday))))
  (if (== _output_get 1800)
    (Actor|DestroyActor)))

(fn ConstructionScript)