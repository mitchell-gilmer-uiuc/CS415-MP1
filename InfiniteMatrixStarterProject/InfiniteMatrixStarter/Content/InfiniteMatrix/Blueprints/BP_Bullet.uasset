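; BP_Bullet is a projectile that credits the player with a score when it overlaps an Enemy.
; Each tick it sweeps along world X at twice the player's ForwardSpeed, scaled by delta time.
; Any overlap destroys the bullet, and an Enemy hit first calls EnemyScore on PlayerPTR without directly destroying that enemy.
; Its lifetime is a Doomsday tick counter that destroys it at 100, so range depends on frame rate.
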(event EventBeginPlay)

(event Collision|EventActorBeginOverlap
  (params (OtherActor :type Actor%20Object%20Reference))
  (Utilities|Casting|CastToEnemy OtherActor
    (:then
      (CallFunction|DefeatEnemy)
      (Actor|DestroyActor))
    (:CastFailed
      (Actor|DestroyActor))))

(event EventTick
  (params (DeltaSeconds :type Float%20%28single-precision%29))
  (Transformation|AddActorWorldOffset (Math|Vector|MakeVector (* (* DeltaSeconds (Variables|/Game/InfiniteMatrix/Blueprints/BP_Player.BP_Player_C|GetForwardSpeed (Variables|Default|GetPlayer_PTR))) 2.0) 0.0 0.0) true)
  (bind _output_get (Variables|Default|SetDoomsday (+ 1 (Variables|Default|GetDoomsday))))
  (if (== _output_get 100)
    (Actor|DestroyActor)))

(fn ConstructionScript)

(fn DefeatEnemy
  (Default|EnemyScore (Variables|Default|GetPlayer_PTR)))